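; Basic melee enemy that chases a target while the player is alive, attacks on arrival and can be killed.
; A successful AI move triggers a delayed explosion effect and sphere overlap at AttackPoint, damaging any player character found, then resuming the chase.
; Incoming damage drains Health; at zero the enemy stops moving, spawns a larger explosion and is destroyed.
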(event `ChasePlayer`
  (params (Target :type "Pawn Object Reference"))
  (bind _asbp_player_character (cast `/Game/Blueprints/Player/BP_PlayerCharacter` (`GameplayStatics.GetPlayerPawn` 0)))
  (if (not (`/Game/Blueprints/Player/BP_PlayerCharacter.PlayerDead` _asbp_player_character))
    (set `self.PlayerTarget` Target)
    (`|AIMoveTo` self (0.0 0.0 0.0) Target
      (:`OnSuccess`
        (`self.AttackPlayer`)))))

(event `self.ReceiveAnyDamage`
  (params (Damage :type "Float (single-precision)") (DamageType :type "DamageType Object Reference") (InstigatedBy :type "Controller Object Reference") (DamageCauser :type "Actor Object Reference"))
  ;[1 1 1] Calculating health loss to death
  (set `self.Health` (- (`self.Health`) Damage))
  (if (<= (`self.Health`) 0.0)
    (`self.Death`)))

(event `AttackPlayer`
  (bind _asbp_player_character (cast `/Game/Blueprints/Player/BP_PlayerCharacter` (`GameplayStatics.GetPlayerPawn` 0)))
  (if (not (`/Game/Blueprints/Player/BP_PlayerCharacter.PlayerDead` _asbp_player_character))
    (`KismetSystemLibrary.Delay` 2.0)
    (`GameplayStatics.SpawnEmitterAtLocation` "/Game/StarterContent/Particles/P_Explosion.P_Explosion" (`SceneComponent.K2_GetComponentLocation` (`self.AttackPoint`)) (struct) (2.0 2.0 2.0) false)
    (bind (_outactors _returnvalue) (`KismetSystemLibrary.SphereOverlapActors` (`SceneComponent.K2_GetComponentLocation` (`self.AttackPoint`)) 50.0 (`|MakeArray` "ObjectTypeQuery3" :!type "EObjectTypeQuery Enum") "/Game/Blueprints/Player/BP_PlayerCharacter.BP_PlayerCharacter_C"))
    (if _returnvalue
      (for _array_element _outactors
        (`GameplayStatics.ApplyDamage` _array_element (`self.Damage`) null self "/Script/Engine.DamageType")
        (`KismetSystemLibrary.Delay` 1.0)
        (`self.ChasePlayer` (`self.PlayerTarget`)))
      (else
        (`self.ChasePlayer` (`self.PlayerTarget`))))))

(event `Death`
  ;[1 1 1] Action on death
  (if (not (`self.Dead`))
    (set `self.Dead` true)
    (`CharacterMovementComponent.DisableMovement` (`self.CharacterMovement`))
    (`Controller.StopMovement` (`self.GetController`))
    (`GameplayStatics.SpawnEmitterAtLocation` "/Game/StarterContent/Particles/P_Explosion.P_Explosion" (`SceneComponent.K2_GetComponentLocation` (`self.CapsuleComponent`)) (struct) (5.0 5.0 5.0) false)
    (`self.K2_DestroyActor`)))

(fn `UserConstructionScript`)