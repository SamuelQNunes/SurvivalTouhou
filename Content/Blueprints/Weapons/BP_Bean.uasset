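; BP_Bean is a bean weapon actor that damages enemies on impact, apparently as a projectile.
; On Hit, it applies its Damage and DamageType to actors tagged Enemy, crediting its owner as the damage causer.
; It destroys itself after any hit, whether or not the target is an enemy.
; BeanT, ChangeBean and IsDead are stub functions that return fixed values.
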(event `self.ReceiveHit`
  (params (MyComp :type "PrimitiveComponent Object Reference") (Other :type "Actor Object Reference") (OtherComp :type "PrimitiveComponent Object Reference") (bSelfMoved :type Boolean) (HitLocation :type "Vector Structure") (HitNormal :type "Vector Structure") (NormalImpulse :type "Vector Structure") (Hit :type "HitResult Structure (by ref)"))
  ;[1 1 1] Applying damage on hit
  (if (`self.ActorHasTag` Other "Enemy")
    (`GameplayStatics.ApplyDamage` Other (`self.Damage`) null (`self.GetOwner`) "/Script/Engine.DamageType")
    (`self.K2_DestroyActor`)
    (else
      (`self.K2_DestroyActor`))))

(fn `BeanT`
  (returns (ShootDelay :type "Float (double-precision)"))
  (return 0.125))

(fn `ChangeBean`
  (returns (CanShoot :type Boolean))
  (return true))

(fn `IsDead`
  (returns (NewParam :type Boolean))
  (return false))

(fn `UserConstructionScript`)